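; BP_StatsSave is a stats save asset holding leaderboard entries, each with a player nickname and best score.
; GetTop5Leads sorts LeadsDataArray in place, highest score first, using nested loops that compare and swap entries.
; Despite its name, it returns the whole array without trimming it to five.
; A disconnected debug loop for printing names and scores never runs.
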(fn `Get Top 5Leads`
  (returns (LeadsDataArray :type "Array of /Game/SaveGame/PlayerScoreStruct Structure"))
  (bind _leadsdataarray (`self.LeadsDataArray`))
  (for (_array_element _array_index) _leadsdataarray
    (for _index (range (`KismetArrayLibrary.Array_Length` _leadsdataarray))
      (bind (_output_playernickname _output_playerbestscore) (break `/Game/SaveGame/PlayerScoreStruct` (`|GetArrayItem` (`self.LeadsDataArray`) _index)))
      (if (> (`.PlayerBestScore_6_3F3AC0174670EC1CC831FABE5B9801BD` (break `/Game/SaveGame/PlayerScoreStruct` _array_element)) _output_playerbestscore)
        (`KismetArrayLibrary.Array_Swap` (`self.LeadsDataArray`) _index _array_index))))
  (return (`self.LeadsDataArray`)))